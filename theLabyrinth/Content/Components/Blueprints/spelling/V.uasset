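; V is a sand-pit hazard that damages overlapping actors and sinks the third-person player before respawning them.
; On SandBox overlap it disables input, and the Sink timeline lerps the player from StartLocaton to a point below it.
; After a short delay the player moves to RespawnPoint and regains input.
; The node capturing the player's location into StartLocaton is unconnected, so the sink uses that variable's existing value.
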(event OnComponentBeginOverlap(sandBox)
  (params (OverlappedComponent :type Primitive%20Component%20Object%20Reference) (OtherActor :type Actor%20Object%20Reference) (OtherComp :type Primitive%20Component%20Object%20Reference) (OtherBodyIndex :type Integer) (bFromSweep :type Boolean) (SweepResult :type Hit%20Result%20Structure%20%28by%20ref%29))
  (Game|Damage|ApplyDamage OtherActor 1.0 0 0)
  (bind _asbp_third_person_character (Utilities|Casting|CastToBP_ThirdPersonCharacter OtherActor)
    (:then
      (Development|PrintString "sand" false)
      (bind _output_get (Variables|Default|SetPlayerRef _asbp_third_person_character))
      (Input|DisableInput (Game|GetPlayerController 0))
      (Variables|Default|SetEndLocation (+ (Variables|Default|GetStartLocaton) (Math|Vector|MakeVector 0.0 0.0 -2e+02)))
      (Development|PrintString "sink" false)
      (bind _newtrack_0 (Timeline|sink Play)
        (:Update
          (Transformation|SetActorLocation (Variables|Default|GetPlayerRef) (Math|Vector|Lerp(Vector) (Variables|Default|GetStartLocaton) (Variables|Default|GetEndLocation) _newtrack_0) false false))
        (:Finished
          (Utilities|FlowControl|Delay 0.3)
          (Transformation|SetActorLocation (Variables|Default|GetPlayerRef) (Variables|Default|GetRespawnPoint) false false)
          (Input|EnableInput (Variables|Default|GetPlayerRef) (Game|GetPlayerController 0)))))
    (:CastFailed
      (Development|PrintString "fail" false))))

(event EventBeginPlay)

(event Collision|EventActorBeginOverlap
  (params (OtherActor :type Actor%20Object%20Reference)))

(event EventTick
  (params (DeltaSeconds :type Float%20%28single-precision%29)))

(fn ConstructionScript)