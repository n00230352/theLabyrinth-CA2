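; BP_Trident is an actor that shows Gawr Gura's trident falling repeatedly in an endless loop.
; On BeginPlay it stores its location and a point 1000 units below, then the Fall timeline lerps the GawrGurasTrident component between them.
; When the timeline finishes, the actor hides, moves back to the start, waits briefly, then reappears and replays the fall.
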(event Collision|EventActorBeginOverlap
  (params (OtherActor :type Actor%20Object%20Reference)))

(event EventTick
  (params (DeltaSeconds :type Float%20%28single-precision%29)))

(event EventBeginPlay
  (Variables|Default|SetInitialPos (Transformation|GetActorLocation))
  (Variables|Default|SetEndPos (+ (Variables|Default|GetInitialPos) (Math|Vector|MakeVector 0.0 0.0 -1e+03)))
  (bind _newtrack_0 (Timeline|Fall Play)
    (:Update
      (Transformation|SetWorldLocation (Variables|Default|Getgawr_guras_trident) (Math|Vector|Lerp(Vector) (Variables|Default|GetInitialPos) (Variables|Default|GetEndPos) _newtrack_0) false false))
    (:Finished
      (Rendering|SetActorHiddenInGame true)
      (Transformation|SetActorLocation (Variables|Default|GetInitialPos) false false)
      (Utilities|FlowControl|Delay 0.3)
      (Rendering|SetActorHiddenInGame false)
      (Timeline|Fall PlayFromStart))))

(fn ConstructionScript)