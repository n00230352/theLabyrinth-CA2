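; BP_Thorn is a thorn actor whose Thorn component shoots out along its local Y axis when play begins.
; BeginPlay caches the component's relative location, derives an end point a short offset away, and plays the Shooting timeline.
; Each timeline update lerps the thorn between those points without sweeping; the file contains no overlap or damage logic.
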(event Collision|EventActorBeginOverlap
  (params (OtherActor :type Actor%20Object%20Reference)))

(event EventTick
  (params (DeltaSeconds :type Float%20%28single-precision%29)))

(event EventBeginPlay
  (Variables|Default|SetStartPos (Variables|/Script/Engine.SceneComponent|GetRelativeLocation (Variables|Default|Getthorn)))
  (Variables|Default|SetEndPos (+ (Variables|Default|GetStartPos) (Math|Vector|MakeVector 0.0 5e+01 0.0)))
  (bind _shooting (Timeline|shooting Play)
    (:Update
      (Transformation|SetRelativeLocation (Variables|Default|Getthorn) (Math|Vector|Lerp(Vector) (Variables|Default|GetStartPos) (Variables|Default|GetEndPos) _shooting) false false))))

(fn ConstructionScript)