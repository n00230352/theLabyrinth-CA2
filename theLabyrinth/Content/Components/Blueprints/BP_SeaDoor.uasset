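; BP_SeaDoor is a puzzle door that opens once three correct shells are selected with no wrong ones.
; RegisterShellSelect counts each correct or wrong selection, then runs CheckPuzzle to test that condition.
; OpenDoor sets IsOpen and destroys the actor rather than animating it.
; Nothing here resets or lowers the counters, so one wrong selection blocks CheckPuzzle from opening the door.
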(event Custom|RegisterShellSelect
  (params (bIsCorrect :type Boolean))
  ;[0.15 0.15 0.15 0.5] Comment
  (if bIsCorrect
    (Variables|Default|SetCorrectSelected (+ (Variables|Default|GetCorrectSelected) 1))
    (CallFunction|CheckPuzzle)
    (else
      (Variables|Default|SetWrongSelected (+ (Variables|Default|GetWrongSelected) 1))
      (CallFunction|CheckPuzzle))))

(event Custom|CheckPuzzle
  ;[0.15 0.15 0.15 0.5] Comment
  (if (and (and (== (Variables|Default|GetCorrectSelected) 3) (== (Variables|Default|GetWrongSelected) 0)) (not (Variables|Default|GetIsOpen)))
    (CallFunction|OpenDoor)))

(event Custom|OpenDoor
  (Variables|Default|SetIsOpen true)
  (Actor|DestroyActor))

(event EventBeginPlay)

(event Collision|EventActorBeginOverlap
  (params (OtherActor :type Actor%20Object%20Reference)))

(event EventTick
  (params (DeltaSeconds :type Float%20%28single-precision%29)))

(fn ConstructionScript)